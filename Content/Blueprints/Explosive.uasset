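; Explosive is a pickup variant that blasts the Ball away when collected, with zero points and no number widget.
; BeginPlay sets the inherited pickup sound and particles to explosion assets and plays a spark sound at its location before calling the parent.
; On pickup by a Ball, it applies a velocity-change radial impulse to the ball mesh from just below itself, then runs the parent pickup logic.
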(event EventBeginPlay
  (Variables|Default|SetUseNumberWidget false)
  (Variables|Default|SetPoints 0)
  (Variables|Default|SetOnPickupSound "/Game/StarterContent/Audio/Explosion01.Explosion01")
  (Variables|Default|SetOnPickUpParticles "/Game/StarterContent/Particles/P_Explosion.P_Explosion")
  (Audio|PlaySoundatLocation "/Game/StarterContent/Audio/Fire_Sparks01_Cue.Fire_Sparks01_Cue" (Transformation|GetActorLocation) "0, 0, 0" 1.0 1.0 0.0 0 0 0)
  (|CallParentFunction))

(event Collision|EventActorBeginOverlap
  (params (OtherActor :type Actor%20Object%20Reference)))

(event EventTick
  (params (DeltaSeconds :type Float%20%28single-precision%29)))

(event EventOnPickUp
  (params (OtherActor :type Object%20Object%20Reference))
  (bind _returnvalue (Transformation|GetActorLocation))
  (bind (_x _y _z) (Math|Vector|BreakVector _returnvalue))
  (bind _asball (Utilities|Casting|CastToBall OtherActor))
  (Physics|AddRadialImpulse (Variables|/Game/Blueprints/Ball.Ball_C|GetBallMesh _asball) (Math|Vector|MakeVector _x _y (+ _z -75.0)) 5e+02 2e+03 "RIF_Constant" true)
  (|CallParentFunction OtherActor))

(fn ConstructionScript
  (|CallParentFunction))