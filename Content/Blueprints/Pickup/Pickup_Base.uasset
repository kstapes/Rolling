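; Base pickup actor that awards Points to a Ball overlapping its sphere, with a 2D sound and particle burst.
; With UseNumberWidget on, it hides the mesh and animates a PickupText widget showing the score; otherwise it destroys itself immediately.
; The overlap event also destroys the actor after a short delay, even when the overlapping actor is not a Ball.
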(event OnComponentBeginOverlap(Sphere)
  (params (OverlappedComponent :type Primitive%20Component%20Object%20Reference) (OtherActor :type Actor%20Object%20Reference) (OtherComp :type Primitive%20Component%20Object%20Reference) (OtherBodyIndex :type Integer) (bFromSweep :type Boolean) (SweepResult :type Hit%20Result%20Structure%20%28by%20ref%29))
  (CallFunction|OnPickUp OtherActor)
  (Utilities|FlowControl|Delay 0.75)
  (Actor|DestroyActor))

(event EventBeginPlay
  (bind _pickuptext (Variables|Default|GetPickupText))
  (Rendering|SetVisibility _pickuptext false false)
  (bind _aspickup_text (Utilities|Casting|CastToPickupText (UserInterface|GetUserWidgetObject _pickuptext)))
  (Variables|/Game/Blueprints/Pickup/PickupText.PickupText_C|SetScoreValue _aspickup_text (Variables|Default|GetPoints)))

(fn ConstructionScript)

(fn OnPickUp
  (params (OtherActor :type Object%20Object%20Reference))
  (bind _asball (Utilities|Casting|CastToBall OtherActor))
  (Default|IncrementScore _asball (Variables|Default|GetPoints))
  (Audio|PlaySound2D (Variables|Default|GetOnPickupSound) 1.0 1.0 0.0 0 0)
  (Effects|SpawnEmitteratLocation (Variables|Default|GetOnPickUpParticles) (Transformation|GetActorLocation))
  (if (Variables|Default|GetUseNumberWidget)
    (Rendering|SetVisibility (Variables|Default|GetPickupText) true false)
    (Rendering|SetVisibility (Variables|Default|GetStaticMesh) false false)
    (bind _aspickup_text (Utilities|Casting|CastToPickupText (UserInterface|GetUserWidgetObject (Variables|Default|GetPickupText))))
    (UserInterface|Animation|PlayAnimation _aspickup_text (Variables|/Game/Blueprints/Pickup/PickupText.PickupText_C|GetPickupAnimation _aspickup_text) 0.0 1 "Forward" 1.0 false)
    (else
      (Actor|DestroyActor))))